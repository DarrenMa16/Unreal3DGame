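; Camera component that lets the game take photos and toggle a gallery widget.
; TakePhoto renders the supplied SceneCapture into a new render target, exports it to the project's Screenshots folder under a timestamped .png name and plays a shutter sound.
; Each file name is appended to the SG_Photos save game, which is created if missing.
; ToggleGallery creates or removes WBP_Gallery and switches input mode, leaving the cursor hidden.
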(event `Take Photo`
  (params (SceneCapture :type "SceneCaptureComponent2D Object Reference"))
  (bind (_returnvalue_year _returnvalue_month _returnvalue_day _returnvalue_hour _returnvalue_minute _returnvalue_second) (`KismetMathLibrary.BreakDateTime` (`KismetMathLibrary.Now`)))
  ; Take Photo
  (bind _returnvalue (`KismetRenderingLibrary.CreateRenderTarget2D` 256 256 "RTF_RGBA8"))
  (bind _output_get (set `SceneCaptureComponent2D.TextureTarget` _returnvalue SceneCapture))
  (`SceneCaptureComponent2D.CaptureScene` SceneCapture)
  (`KismetSystemLibrary.Delay` 0.2)
  (bind _output_get_2 (set `self.Photo` _output_get))
  (bind _output_get_3 (set `self.FileName` (`KismetStringLibrary.Concat_StrStr` (`KismetTextLibrary.Conv_TextToString` (`|FormatText` "MaxAsplandPhoto{DD}{MM}{YYYY}{HH}{MI}{SS}" (`KismetTextLibrary.Conv_IntToText` _returnvalue_day false false 2) (`KismetTextLibrary.Conv_IntToText` _returnvalue_month false false 2) (`KismetTextLibrary.Conv_IntToText` _returnvalue_year false false 2) (`KismetTextLibrary.Conv_IntToText` _returnvalue_hour false false 2) (`KismetTextLibrary.Conv_IntToText` _returnvalue_minute false false 2) (`KismetTextLibrary.Conv_IntToText` _returnvalue_second false false 2))) ".png")))
  (`KismetSystemLibrary.Delay` 0.5)
  (`KismetRenderingLibrary.ExportRenderTarget` _output_get_2 (`KismetStringLibrary.Concat_StrStr` (`KismetSystemLibrary.GetProjectDirectory`) "Screenshots/") _output_get_3)
  (set `self.Photo` null)
  (`GameplayStatics.PlaySound2D` "/Game/Camera/CamShutter_Fixed.CamShutter_Fixed" 2.0 1.0 0.0 null null)
  ; Save the Unique File Name
  (bind _returnvalue_2 (`GameplayStatics.DoesSaveGameExist` "SG_Photos"))
  (if _returnvalue_2
    (bind _returnvalue_3 (`GameplayStatics.LoadGameFromSlot` "SG_Photos"))
    (bind _assg_photos (cast `/Game/Camera/SG_Photos` _returnvalue_3)
      (:`then`
        (bind _output_get_4 (set `self.As SG Photos` _assg_photos))
        (`KismetArrayLibrary.Array_Add` (`/Game/Camera/SG_Photos.PhotoFileNames` _output_get_4) (`self.FileName`))
        (`GameplayStatics.SaveGameToSlot` (`self.As SG Photos`) "SG_Photos" :!label _label)
        (`KismetSystemLibrary.PrintString` "Photo Taken"))
      (:`CastFailed`
        (`KismetSystemLibrary.PrintString` "Failed")))
    (else
      (bind _returnvalue_4 (`GameplayStatics.CreateSaveGameObject` "/Game/Camera/SG_Photos.SG_Photos_C"))
      (bind _output_get_5 (set `self.As SG Photos` _returnvalue_4))
      (`KismetArrayLibrary.Array_Add` (`/Game/Camera/SG_Photos.PhotoFileNames` _output_get_5) (`self.FileName`))
      (goto _label))))

(event `ToggleGallery`
  (bind _returnvalue (`GameplayStatics.GetPlayerController` 0))
  (bind _returnvalue_2 (`GameplayStatics.GetPlayerController` 0))
  ; Toggle Gallery
  (bind _gallery (`self.Gallery`)
    (:`then`
      (`Widget.RemoveFromParent` _gallery)
      (set `self.Gallery` null)
      (`WidgetBlueprintLibrary.SetInputMode_GameOnly` _returnvalue_2)
      (set `PlayerController.bShowMouseCursor` false _returnvalue_2))
    (:`else`
      (bind _returnvalue_3 (`|CreateWidget` "/Game/Camera/WBP_Gallery.WBP_Gallery_C"))
      (bind _output_get (set `self.Gallery` _returnvalue_3))
      (`UserWidget.AddToViewport` _output_get 0)
      (`WidgetBlueprintLibrary.SetInputMode_GameAndUIEx` _returnvalue _output_get)
      (set `PlayerController.bShowMouseCursor` false _returnvalue))))