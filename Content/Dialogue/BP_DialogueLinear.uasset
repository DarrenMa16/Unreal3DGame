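; BP_DialogueLinear is an actor that manages a linear dialogue widget, advanced with the Q key.
; On BeginPlay it enables input from player 0, and Q calls Advance on the widget while it is visible.
; Logic to create WBP_DialogueLinear from a DialogueTable and bind its finished event is disconnected, and the Box overlap event is empty.
; HandleDialogueFinished removes the widget and clears the visible flag.
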(event `self.Box.OnComponentBeginOverlap`
  (params (OverlappedComponent :type "PrimitiveComponent Object Reference") (OtherActor :type "Actor Object Reference") (OtherComp :type "PrimitiveComponent Object Reference") (OtherBodyIndex :type Integer) (bFromSweep :type Boolean) (SweepResult :type "HitResult Structure (by ref)")))

(event `self.ReceiveBeginPlay`
  ; If you want it to happen on a key press instead -> get the input from player controller
  (`self.EnableInput` (`GameplayStatics.GetPlayerController` 0)))

(event `HandleDialogueFinished`
  (`Widget.RemoveFromParent` (`self.Dialogue Widget`))
  (set `self.isVisible` false)
  (if true
    _))

(event `Key|Q`
  (params (Key :type "Key Structure"))
  ; Press Q to Advance Dialogue
  (:`Pressed`
    (if (`self.isVisible`)
      (`/Game/Dialogue/WBP_DialogueLinear.Advance` (`self.Dialogue Widget`)))))

(fn `BP_DialogueLinear_AutoGenFunc`)

(fn `UserConstructionScript`)